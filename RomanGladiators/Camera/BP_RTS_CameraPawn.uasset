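; RTS camera pawn that pans, zooms and rotates the view within map bounds.
; Each Tick adds mouse screen-edge direction to directional pan flags, moves along world XY regardless of yaw, then clamps position to min/max limits.
; Spring arm length and actor yaw then ease toward their targets with FInterpTo.
; The pan flags and zoom/yaw targets are only read here, never set.
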(event `self.ReceiveTick`
  (params (DeltaSeconds :type "Float (single-precision)"))
  (`self.PanByInput`)
  (`self.ClampToBounds`)
  (`self.ApplyZoomTarget`)
  (`self.ApplyYawTarget`))

(fn `ApplyYawTarget`
  (`self.K2_SetActorRotation` (`KismetMathLibrary.MakeRotator` (.roll (`self.K2_GetActorRotation`)) (.pitch (`self.K2_GetActorRotation`)) (`KismetMathLibrary.FInterpTo` (.yaw (`self.K2_GetActorRotation`)) (`self.YawTarget`) (`GameplayStatics.GetWorldDeltaSeconds`) (`self.RotateInterpSpeed`)))))

(fn `ApplyZoomTarget`
  (bind _springarm (`self.SpringArm`))
  (set `SpringArmComponent.TargetArmLength` (`KismetMathLibrary.FInterpTo` (`SpringArmComponent.TargetArmLength` _springarm) (`self.ZoomTargetArmLength`) (`GameplayStatics.GetWorldDeltaSeconds`) (`self.ZoomInterpSpeed`)) _springarm))

(fn `ClampToBounds`
  (`self.K2_SetActorLocation` (`KismetMathLibrary.MakeVector` (`KismetMathLibrary.FClamp` (.x (`self.K2_GetActorLocation`)) (`self.MinX`) (`self.MaxX`)) (`KismetMathLibrary.FClamp` (.y (`self.K2_GetActorLocation`)) (`self.MinY`) (`self.MaxY`)) (.z (`self.K2_GetActorLocation`)))))

(fn `ComputeEdgeDirection`
  (returns (EdgeDirection :type "Vector2D Structure"))
  (bind _edgemarginpx (`self.EdgeMarginPX`))
  (bind _edgemarginpx_2 (`self.EdgeMarginPX`))
  (bind (_x _y) (`KismetMathLibrary.BreakVector2D` (`WidgetLayoutLibrary.GetViewportSize`)))
  (bind _returnvalue (`WidgetLayoutLibrary.GetMousePositionOnViewport`))
  (bind (_x_2 _y_2) (`KismetMathLibrary.BreakVector2D` _returnvalue))
  (bind _output_get (set `self.EdgeDirection` (`KismetMathLibrary.Normal2D` (`KismetMathLibrary.MakeVector2D` (`KismetMathLibrary.SelectFloat` 1.0 (`KismetMathLibrary.SelectFloat` -1.0 0.0 (< _x_2 _edgemarginpx_2)) (> _x_2 (- _x _edgemarginpx))) (`KismetMathLibrary.SelectFloat` -1.0 (`KismetMathLibrary.SelectFloat` 1.0 0.0 (< _y_2 _edgemarginpx_2)) (> _y_2 (- _y _edgemarginpx)))))))
  (return _output_get))

(fn `PanByInput`
  (returns (ReturnValue :type "Vector Structure"))
  (bind _edgedirection (`self.ComputeEdgeDirection`))
  (bind (_returnvalue_x _returnvalue_y) (`KismetMathLibrary.BreakVector2D` (* (+ _edgedirection (`KismetMathLibrary.MakeVector2D` (+ (`KismetMathLibrary.SelectFloat` 1.0 0.0 (`self.IsPanningRight`)) (`KismetMathLibrary.SelectFloat` -1.0 0.0 (`self.IsPanningLeft`))) (+ (`KismetMathLibrary.SelectFloat` 1.0 0.0 (`self.IsPanningForward`)) (`KismetMathLibrary.SelectFloat` -1.0 0.0 (`self.IsPanningBackward`))))) (* (`GameplayStatics.GetWorldDeltaSeconds`) (`self.PanSpeedUUps`)))))
  (bind _returnvalue (+ (`KismetMathLibrary.MakeVector` _returnvalue_x _returnvalue_y) (`self.K2_GetActorLocation`)))
  (`self.K2_SetActorLocation` _returnvalue)
  (return _returnvalue))

(fn `UserConstructionScript`)