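; BP_UnitPawn is a gladiator unit pawn with functions for selection, highlighting and move commands.
; ReceiveCommand passes a target location to the pawn's BP_GladiatorAIController through CommandMoveTo.
; SetSelected always sets IsSelected to true, then calls selected or deselected visual events, which are empty here.
; Highlight only assigns dice material variables based on IsHighlighted, without applying them to a mesh.
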(event `ApplySelectedVisuals`)

(event `ApplyDeselectedVisuals`)

(fn `Highlight`
  (if (`self.IsHighlighted`)
    (set `self.HighlightMaterial` "/Game/Dice/Materials/M_Dice_Yellow.M_Dice_Yellow")
    (else
      (set `self.BaseMaterial` "/Game/Dice/Materials/M_Dice_White.M_Dice_White"))))

(fn `ReceiveCommand`
  (params (TargetLocation :type "Vector Structure"))
  (bind _asbp_gladiator_aicontroller (cast `/Game/RomanGladiators/GladiatorCharacters/BP_GladiatorAIController` (`self.GetController`)))
  (`/Game/RomanGladiators/GladiatorCharacters/BP_GladiatorAIController.CommandMoveTo` _asbp_gladiator_aicontroller TargetLocation))

(fn `SetSelected`
  (params (NewSelected :type Boolean))
  (set `self.IsSelected` true)
  (if NewSelected
    (`self.ApplySelectedVisuals`)
    (else
      (`self.ApplyDeselectedVisuals`))))

(fn `UserConstructionScript`)