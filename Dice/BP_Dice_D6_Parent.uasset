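; Parent Blueprint for a physics-driven six-sided die that detects and prints the face it lands on.
; RollDie applies random linear and angular impulses and clears the FaceValues array that the top-face lookup reads.
; Tick times low linear velocity, then calls ComputeTopFace and prints the result every frame while settled.
; ComputeTopFace dots world-space face normals against up, keeping a MaxDot that is never reset here.
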(event `self.ReceiveTick`
  (params (DeltaSeconds :type "Float (single-precision)"))
  (set `self.Delta Seconds` DeltaSeconds)
  (bind _returnvalue (`PrimitiveComponent.GetPhysicsLinearVelocity` (`self.SM_D6Die`) "None"))
  (if (< (`KismetMathLibrary.VSize` _returnvalue) 1.0)
    (bind _output_get (set `self.SettleTimer` (+ (`self.SettleTimer`) (`self.Delta Seconds`))))
    (if (> _output_get 0.5)
      (`self.ComputeTopFace`)
      (`KismetSystemLibrary.PrintString` (`KismetStringLibrary.Concat_StrStr` "The Top Face value is: " (`KismetStringLibrary.Conv_IntToString` (`self.TopValue`))) true true (struct :`A` 1.0) 10.0))
    (else
      (set `self.SettleTimer` 0.0))))

(event `Key|SpaceBar`
  (params (Key :type "Key Structure")))

(fn `ComputeTopFace`
  (for (_array_element _array_index) (`self.FaceNormals`)
    (bind _returnvalue (`KismetMathLibrary.Dot_VectorVector` (`KismetMathLibrary.TransformDirection` (`SceneComponent.K2_GetComponentToWorld` (`self.SM_D6Die`)) _array_element) (`KismetMathLibrary.MakeVector` 0.0 0.0 1.0)))
    (if (> _returnvalue (`self.MaxDot`))
      (set `self.MaxDot` _returnvalue)
      (set `self.MaxIndex` _array_index)))
  (set `self.TopValue` (`|GetArrayItem` (`self.FaceValues`) (`self.MaxIndex`))))

(fn `RollDie`
  (`KismetArrayLibrary.Array_Clear` (`self.FaceValues`))
  (set `self.bRolling` true)
  (set `self.LastBelowThresholdTime` 0.0)
  (`PrimitiveComponent.AddImpulse` (`self.SM_D6Die`) (* (`KismetMathLibrary.RandomUnitVector`) (`self.ImpulseMagnitude`)) "None" true)
  (`PrimitiveComponent.AddAngularImpulseInDegrees` (`self.SM_D6Die`) (* (`KismetMathLibrary.RandomUnitVector`) (`self.TorqueMagnitude`)) "None" true))

(fn `UserConstructionScript`)